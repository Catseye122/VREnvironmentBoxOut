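; BP_Potion is a potion actor that changes its glass material when it touches a flower powder.
; On a Box begin overlap, it checks poppy, blue, purple, violet and white powders in order, and the first match sets the StaticMesh material.
; Each check tests only the single instance returned by GetActorOfClass, ignoring the event's overlapping actor.
; Each match also creates a dynamic material instance that goes unused.
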(event `self.Box.OnComponentBeginOverlap`
  (params (OverlappedComponent :type "PrimitiveComponent Object Reference") (OtherActor :type "Actor Object Reference") (OtherComp :type "PrimitiveComponent Object Reference") (OtherBodyIndex :type Integer) (bFromSweep :type Boolean) (SweepResult :type "HitResult Structure (by ref)"))
  (bind _returnvalue (`GameplayStatics.GetActorOfClass` "/Game/Blueprints/BP_poppypowder.BP_poppypowder_C"))
  (if (`self.IsOverlappingActor` _returnvalue)
    (`KismetMaterialLibrary.CreateDynamicMaterialInstance` (`PrimitiveComponent.GetMaterial` (`self.StaticMesh`) 0))
    (`PrimitiveComponent.SetMaterial` (`self.StaticMesh`) 0 "/Game/GardenAssets/PoppyGlass_Mat.PoppyGlass_Mat")
    (else
      (bind _returnvalue_2 (`GameplayStatics.GetActorOfClass` "/Game/Blueprints/BP_bluepowder.BP_bluepowder_C"))
      (if (`self.IsOverlappingActor` _returnvalue_2)
        (`KismetMaterialLibrary.CreateDynamicMaterialInstance` (`PrimitiveComponent.GetMaterial` (`self.StaticMesh`) 0))
        (`PrimitiveComponent.SetMaterial` (`self.StaticMesh`) 0 "/Game/GardenAssets/BellFlwoer_Mat.BellFlwoer_Mat")
        (else
          (bind _returnvalue_3 (`GameplayStatics.GetActorOfClass` "/Game/Blueprints/BP_purplepowder.BP_purplepowder_C"))
          (if (`self.IsOverlappingActor` _returnvalue_3)
            (`KismetMaterialLibrary.CreateDynamicMaterialInstance` (`PrimitiveComponent.GetMaterial` (`self.StaticMesh`) 0))
            (`PrimitiveComponent.SetMaterial` (`self.StaticMesh`) 0 "/Game/GardenAssets/DarkPurpleGlass_Mat.DarkPurpleGlass_Mat")
            (else
              (bind _returnvalue_4 (`GameplayStatics.GetActorOfClass` "/Game/Blueprints/BP_violetpowder.BP_violetpowder_C"))
              (if (`self.IsOverlappingActor` _returnvalue_4)
                (`KismetMaterialLibrary.CreateDynamicMaterialInstance` (`PrimitiveComponent.GetMaterial` (`self.StaticMesh`) 0))
                (`PrimitiveComponent.SetMaterial` (`self.StaticMesh`) 0 "/Game/GardenAssets/LightPrupleGlass_Mat.LightPrupleGlass_Mat")
                (else
                  (bind _returnvalue_5 (`GameplayStatics.GetActorOfClass` "/Game/Blueprints/BP_whitepowder.BP_whitepowder_C"))
                  (if (`self.IsOverlappingActor` _returnvalue_5)
                    (`KismetMaterialLibrary.CreateDynamicMaterialInstance` (`PrimitiveComponent.GetMaterial` (`self.StaticMesh`) 0))
                    (`PrimitiveComponent.SetMaterial` (`self.StaticMesh`) 0 "/Game/GardenAssets/Glass_Mat.Glass_Mat")))))))))))

(fn `UserConstructionScript`)