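; BP_flower_13_07 is a flower ingredient that grinds into violet powder in a mortar and pestle.
; On an overlap or hit event, it looks up one mortar and one pestle by class and checks that it overlaps both.
; If so, it destroys itself and spawns BP_violetpowder at the mortar's root transform, ignoring collision.
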(event `self.ReceiveActorBeginOverlap`
  (params (OtherActor :type "Actor Object Reference"))
  (bind _returnvalue (`GameplayStatics.GetActorOfClass` "/Game/Blueprints/BP_MortarV2.BP_MortarV2_C" :!label _label))
  (if (`self.IsOverlappingActor` _returnvalue)
    (bind _returnvalue_2 (`GameplayStatics.GetActorOfClass` "/Game/Blueprints/BP_PestleV2.BP_PestleV2_C"))
    (if (`self.IsOverlappingActor` _returnvalue_2)
      (`self.K2_DestroyActor`)
      (`|SpawnActorFromClass` "/Game/Blueprints/BP_violetpowder.BP_violetpowder_C" (`SceneComponent.K2_GetComponentToWorld` (`Actor.RootComponent` _returnvalue)) "AlwaysSpawn" "MultiplyWithRoot" null null))))

(event `self.ReceiveHit`
  (params (MyComp :type "PrimitiveComponent Object Reference") (Other :type "Actor Object Reference") (OtherComp :type "PrimitiveComponent Object Reference") (bSelfMoved :type Boolean) (HitLocation :type "Vector Structure") (HitNormal :type "Vector Structure") (NormalImpulse :type "Vector Structure") (Hit :type "HitResult Structure (by ref)"))
  (goto _label))

(fn `UserConstructionScript`)